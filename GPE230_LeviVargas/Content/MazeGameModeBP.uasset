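; Game mode for a maze game that plays starter music on begin play and provides level flow and pause functions.
; LoadNextLevel matches the current level name against the ordered GameLevels array and opens the following entry, falling back to the main menu when none is found.
; Other functions restart the current level by name, load the main menu, and pause or resume the game.
; Save logic for the furthest completed level is present but disconnected.
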(event `self.ReceiveBeginPlay`
  (`GameplayStatics.PlaySound2D` "/Game/Audio/Starter_Music01.Starter_Music01" 1.0 1.0 0.0 null null))

(fn `Load Main Menu`
  (`GameplayStatics.OpenLevel` "MainMenuLevel")
  (return))

(fn `Load Next Level`
  (for _index (range 1 (+ (`KismetArrayLibrary.Array_LastIndex` (`self.GameLevels`)) 1))
    (set `self.Level Index` _index)
    (bind _returnvalue (`GameplayStatics.GetCurrentLevelName` true))
    (if (`KismetStringLibrary.EqualEqual_StrStr` _returnvalue (`KismetSystemLibrary.GetObjectName` (`|ConvertAsset` (`|GetArrayItem` (`self.GameLevels`) (- (`self.Level Index`) 1)))))
      (`GameplayStatics.OpenLevelBySoftObjectPtr` (`|GetArrayItem` (`self.GameLevels`) (`self.Level Index`)))
      (return)))
  (`self.Load Main Menu`)
  (return))

(fn `PauseGame`
  (`GameplayStatics.SetGamePaused` true)
  (return))

(fn `Restart Level`
  (bind _returnvalue (`GameplayStatics.GetCurrentLevelName` true))
  (`GameplayStatics.OpenLevel` (`KismetStringLibrary.Conv_StringToName` _returnvalue))
  (return))

(fn `ResumeGame`
  (`GameplayStatics.SetGamePaused` false)
  (return))

(fn `UserConstructionScript`)