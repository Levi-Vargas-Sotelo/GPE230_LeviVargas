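; Player character for a maze game, with an area stun ability against enemies and access to the pause menu.
; Stun plays sound and particles, then sphere-traces around the character and calls Stunned on NPCEnemyBP hits, gated by a cooldown that Tick counts down and a getter exposes.
; Pause opens the menu widget, shows the cursor and pauses through MazeGameModeBP.
; The M key makes the character damage itself.
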(event `self.ReceiveTick`
  (params (DeltaSeconds :type "Float (single-precision)"))
  (if (> (`self.StunCooldown`) 0.0)
    (set `self.StunCooldown` (- (`self.StunCooldown`) DeltaSeconds))))

(event `Key|M`
  (params (Key :type "Key Structure"))
  (:`Pressed`
    (`GameplayStatics.ApplyDamage` self 10.0)))

(event `InputAction|Stun`
  (params (Key :type "Key Structure"))
  (bind _returnvalue (`self.K2_GetActorLocation`))
  (:`Pressed`
    (if (<= (`self.StunCooldown`) 0.0)
      (set `self.StunCooldown` (`self.TimeBetweenStuns`))
      (`GameplayStatics.PlaySoundAtLocation` "/Game/Audio/SFX_Stun.SFX_Stun" (`self.K2_GetActorLocation`) (struct) 1.0 1.0 0.0 null null null null)
      (`self.ActivateStunParticleSystem`)
      (bind _outhits (`KismetSystemLibrary.SphereTraceMultiForObjects` _returnvalue _returnvalue (`self.StunTraceRadius`) (`self.StunTraceTypes`)))
      (for _array_element _outhits
        (bind _asnpcenemy_bp (cast `/Game/NPCEnemyBP` (`.HitActor` (`GameplayStatics.BreakHitResult` _array_element))))
        (`/Game/NPCEnemyBP.Stunned` _asnpcenemy_bp)))))

(event `InputAction|Pause`
  (params (Key :type "Key Structure"))
  (:`Pressed`
    (bind _returnvalue (`|CreateWidget` "/Game/UI/PauseMenuWidgetBP.PauseMenuWidgetBP_C"))
    (`UserWidget.AddToViewport` _returnvalue 0)
    (set `PlayerController.bShowMouseCursor` true (`GameplayStatics.GetPlayerController` 0))
    (bind _asmaze_game_mode_bp (cast `/Game/MazeGameModeBP` (`GameplayStatics.GetGameMode`)))
    (`/Game/MazeGameModeBP.PauseGame` _asmaze_game_mode_bp)))

(fn `GetStunCooldown`
  (returns (CurrentCooldown :type "Float (double-precision)"))
  (return (`self.StunCooldown`)))

(fn `UserConstructionScript`)