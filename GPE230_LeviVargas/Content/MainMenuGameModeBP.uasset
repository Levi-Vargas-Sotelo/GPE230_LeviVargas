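; Main menu game mode that opens the front end and provides the actions for starting the game and showing sub-menus.
; On BeginPlay it creates the main menu widget, shows the mouse cursor and plays the menu music.
; Separate functions create and add the level select and options widgets to the viewport, while StartTheGame opens the first level by name.
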(event `self.ReceiveBeginPlay`
  (`self.DisplayMainMenu`)
  (set `PlayerController.bShowMouseCursor` true (`GameplayStatics.GetPlayerController` 0))
  (`GameplayStatics.PlaySound2D` "/Game/Audio/Music_MainMenu.Music_MainMenu" 1.0 1.0 0.0 null null))

(fn `DisplayMainMenu`
  (bind _returnvalue (`|CreateWidget` "/Game/UI/MainMenuWidgetBP.MainMenuWidgetBP_C"))
  (`UserWidget.AddToViewport` _returnvalue 0))

(fn `DisplayOptions`
  (bind _returnvalue (`|CreateWidget` "/Game/UI/OptionsWidgetBP.OptionsWidgetBP_C"))
  (`UserWidget.AddToViewport` _returnvalue 0))

(fn `DisplaySelectLevel`
  (bind _returnvalue (`|CreateWidget` "/Game/UI/SelectLevelWidgetBP.SelectLevelWidgetBP_C"))
  (`UserWidget.AddToViewport` _returnvalue 0))

(fn `StartTheGame`
  (`GameplayStatics.OpenLevel` "Level1")
  (return))

(fn `UserConstructionScript`)